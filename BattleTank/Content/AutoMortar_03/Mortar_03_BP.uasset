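; Mortar_03_BP is an auto mortar Blueprint with an aiming component and a health bar widget.
; On BeginPlay it initializes TankAiming with its Barrel and Dome as the barrel and turret.
; It then casts the widget component's user widget to HealthBar and sets itself as that widget's ParentTank, reusing the tank aiming and health bar setup.
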(event `self.ReceiveBeginPlay`
  (`TankAimingComponent.Initialize` (`self.TankAiming`) (`self.Barrel`) (`self.Dome`))
  (`self.InitializeHealthBarWidget`))

(fn `InitializeHealthBarWidget`
  (bind _ashealth_bar (cast `/Game/UI/HealthBar` (`WidgetComponent.GetUserWidgetObject` (`self.HealthBarWidget`))))
  (set `/Game/UI/HealthBar.ParentTank` self _ashealth_bar)
  (return))

(fn `UserConstructionScript`)